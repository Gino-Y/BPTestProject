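; BP_FlowControl is a Blueprint test of flow-control nodes, printing whether variable A is greater than B.
; Tick runs the comparison Branch every frame and prints "true" or "false".
; Pressing or releasing key 1 uses a Sequence to set A, then re-enters the same Branch.
; RetriggerableDelay and MultiGate nodes sit unconnected and never run.
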(event EventBeginPlay)

(event Collision|EventActorBeginOverlap
  (params (OtherActor :type Actor%20Object%20Reference)))

(event EventTick
  (params (DeltaSeconds :type Float%20%28single-precision%29))
  (if (> (Variables|Default|Geta) (Variables|Default|Getb)) ; 分支节点
    (Development|PrintString "true")
    (else
      (Development|PrintString "false"))))

(event Input|KeyboardEvents|1
  (params (Key :type Key%20Structure :default "None"))
  (:Pressed
    (Utilities|FlowControl|Sequence
      (:then_0
        (Variables|Default|Seta 3))
      (:then_1
        (if (> (Variables|Default|Geta) (Variables|Default|Getb)) :!label _label ; 分支节点
          (Development|PrintString "true")
          (else
            (Development|PrintString "false"))))))
  (:Released
    (Utilities|FlowControl|Sequence
      (:then_0
        (Variables|Default|Seta 1))
      (:then_1
        (goto _label)))))

(fn ConstructionScript)