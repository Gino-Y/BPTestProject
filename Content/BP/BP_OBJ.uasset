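; BP_OBJ is a test actor that drives a point light and prints an object's name.
; The construction script sets the light's intensity and applies the color from its NewLightColor variable.
; On BeginPlay it prints the name of the object held in Obj to the screen.
; Key 1 turns the light red when pressed and green-cyan when released, keeping the same intensity.
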(event EventBeginPlay
  (Development|PrintString (Utilities|GetObjectName (Variables|Default|GetObj)) true true "(R=0.000000,G=0.660000,B=1.000000,A=1.000000)" 1e+01))

(event Collision|EventActorBeginOverlap
  (params (OtherActor :type Actor%20Object%20Reference)))

(event EventTick
  (params (DeltaSeconds :type Float%20%28single-precision%29)))

(event Input|KeyboardEvents|1
  (params (Key :type Key%20Structure :default "None"))
  (bind _pointlight (Variables|Default|GetPointLight))
  (:Pressed
    (Rendering|Components|Light|SetIntensity _pointlight 1e+04)
    (Rendering|Components|Light|SetLightColor _pointlight "(R=1.000000,G=0.000000,B=0.000000,A=1.000000)" true))
  (:Released
    (Rendering|Components|Light|SetIntensity _pointlight 1e+04)
    (Rendering|Components|Light|SetLightColor _pointlight "(R=0.000000,G=1.000000,B=0.397064,A=1.000000)" true)))

(fn ConstructionScript
  (bind _pointlight (Variables|Default|GetPointLight))
  (Rendering|Components|Light|SetIntensity _pointlight 1e+04)
  (Rendering|Components|Light|SetLightColor _pointlight (Variables|light|GetNew%20Light%20Color) true))