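; Test Blueprint that animates the intensity of a referenced light over time with a float curve, in a repeating cycle.
; Each Tick samples MyCurve at ElapsedTime and uses it to lerp between the Intensity variable and a fixed maximum.
; ElapsedTime accumulates delta time and resets one second after passing CurveLenght.
; The node that copies the light's own intensity into Intensity is unconnected and never runs.
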(event EventBeginPlay)

(event Collision|EventActorBeginOverlap
  (params (OtherActor :type Actor%20Object%20Reference)))

(event EventTick
  (params (DeltaSeconds :type Float%20%28single-precision%29))
  (Utilities|FlowControl|Sequence
    (:then_0
      (Rendering|Components|Light|SetIntensity (Variables|/Script/Engine.Light|GetLightComponent (Variables|Default|GetMyLight)) (Math|Float|Lerp (Variables|Default|GetIntensity) 3e+01 (Math|Curves|GetFloatValue (Variables|Default|GetMyCurve) (Variables|Default|GetElapsedTime)))))
    (:then_1
      (bind _output_get (Variables|Default|SetElapsedTime (+ DeltaSeconds (Variables|Default|GetElapsedTime))))
      (if (> _output_get (Variables|Default|GetCurveLenght))
        (Utilities|FlowControl|Delay 1.0)
        (Variables|Default|SetElapsedTime 0.0)))))

(fn ConstructionScript)