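; BP_Time is an actor that displays a count-up minutes:seconds timer on four text render components, one per digit.
; Tick feeds a one-second Delay that paces increments of the seconds digit.
; Nested branches carry each digit into the next, rolling over at ten for units and six for tens, so the display wraps after 59:59.
; An unfinished Num helper for updating a digit is never called.
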(event EventBeginPlay)

(event Collision|EventActorBeginOverlap
  (params (OtherActor :type Actor%20Object%20Reference)))

(event EventTick
  (params (DeltaSeconds :type Float%20%28single-precision%29))
  (Utilities|FlowControl|Delay 1.0)
  (bind _output_get (Variables|Default|Setvar-s (+ (Variables|Default|Getvar-s) 1)))
  (if (>= _output_get 10)
    (bind _output_get_2 (Variables|Default|Setvar-s 0))
    (Rendering|Components|TextRender|SetText (Variables|Default|Gets) (Utilities|Text|ToText(Integer) _output_get_2))
    (bind _output_get_3 (Variables|Default|Setvar-ss (+ (Variables|Default|Getvar-ss) 1)))
    (if (>= _output_get_3 6)
      (bind _output_get_4 (Variables|Default|Setvar-ss 0))
      (Rendering|Components|TextRender|SetText (Variables|Default|Getss) (Utilities|Text|ToText(Integer) _output_get_4))
      (bind _output_get_5 (Variables|Default|Setvar-m (+ (Variables|Default|Getvar-m) 1)))
      (if (>= _output_get_5 10)
        (bind _output_get_6 (Variables|Default|Setvar-m 0))
        (Rendering|Components|TextRender|SetText (Variables|Default|Getm) (Utilities|Text|ToText(Integer) _output_get_6))
        (bind _output_get_7 (Variables|Default|Setvar-mm (+ (Variables|Default|Getvar-mm) 1)))
        (if (>= _output_get_7 6)
          (bind _output_get_8 (Variables|Default|Setvar-mm 0))
          (Rendering|Components|TextRender|SetText (Variables|Default|Getmm) (Utilities|Text|ToText(Integer) _output_get_8))
          (else
            (Rendering|Components|TextRender|SetText (Variables|Default|Getmm) (Utilities|Text|ToText(Integer) _output_get_7))))
        (else
          (Rendering|Components|TextRender|SetText (Variables|Default|Getm) (Utilities|Text|ToText(Integer) _output_get_5))))
      (else
        (Rendering|Components|TextRender|SetText (Variables|Default|Getss) (Utilities|Text|ToText(Integer) _output_get_3))))
    (else
      (Rendering|Components|TextRender|SetText (Variables|Default|Gets) (Utilities|Text|ToText(Integer) _output_get)))))

(fn ConstructionScript)

(fn Num
  (params (Var-n :type Integer) (Text%20Render :type Text%20Render%20Component%20Object%20Reference) (wei :type Integer))
  (bind _output_get (Variables|Default|SetVar-n (+ Var-n 1)))
  (Rendering|Components|TextRender|SetText Text%20Render (Utilities|Text|ToText(Integer) _output_get)))