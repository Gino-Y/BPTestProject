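; BP_Array is a sandbox Blueprint that demonstrates array operations on MyArray through keyboard input and screen prints.
; Key 3 prints each element and index, breaks out of the loop on reaching a set value, then prints an end-of-traversal message.
; Key 4 shuffles the array.
; Other examples, such as add, insert, resize, remove, find and plain loops, sit in the graph but never run.
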(event EventBeginPlay)

(event Collision|EventActorBeginOverlap
  (params (OtherActor :type Actor%20Object%20Reference)))

(event EventTick
  (params (DeltaSeconds :type Float%20%28single-precision%29)))

(event Input|KeyboardEvents|3
  (params (Key :type Key%20Structure :default "None"))
  (:Pressed
    ;[0.1686 0.4752 1] 碰到相应值即结束遍历
    (bind (_array_element _array_index) (Utilities|Array|ForEachLoopwithBreak (Variables|Default|GetMy%20Array) :!label _label)
      (:LoopBody
        (if (== _array_element 13.0)
          (goto _label Break)
          (else
            (Development|PrintString (Utilities|String|Append "element:" (Utilities|String|ToString(Float) _array_element) "index:" (Utilities|String|ToString(Integer) _array_index))))))
      (:Completed
        (Development|PrintString "遍历结束")))))

(event Input|KeyboardEvents|4
  (params (Key :type Key%20Structure :default "None"))
  (:Pressed
    (Utilities|Array|Shuffle (Variables|Default|GetMy%20Array)) ; 打乱值的位置
  ))

(fn ConstructionScript)